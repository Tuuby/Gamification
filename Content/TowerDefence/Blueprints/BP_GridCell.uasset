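; BP_GridCell is a Tower Defence grid cell actor that holds one placed component.
; PlaceComponent spawns the given actor class with the given rotation, only when the cell's PlacedActor is empty, and stores the result there.
; GetComponentSpawn supplies the location from ComponentArrow's world position, and spawning ignores collisions.
; The event graph and construction script contain no logic.
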(event EventBeginPlay)

(event Collision|EventActorBeginOverlap
  (params (OtherActor :type Actor%20Object%20Reference)))

(event EventTick
  (params (DeltaSeconds :type Float%20%28single-precision%29)))

(fn ConstructionScript)

(fn PlaceComponent
  (params (ComponentClass :type Actor%20Class%20Reference) (Rotation :type Rotator))
  (if (== (Variables|Default|GetPlacedActor) 0)
    (bind _spawnposition (CallFunction|GetComponentSpawn))
    (bind _returnvalue (Game|SpawnActorfromClass ComponentClass (Math|Transform|MakeTransform _spawnposition Rotation) "AlwaysSpawn" "MultiplyWithRoot" 0 0))
    (Variables|Default|SetPlacedActor _returnvalue)))

(fn GetComponentSpawn
  (return (Transformation|GetWorldLocation (Variables|Default|GetComponentArrow))))