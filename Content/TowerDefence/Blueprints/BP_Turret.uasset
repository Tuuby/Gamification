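; Tower defence turret that fires projectiles when its wired signal input switches on.
; Tick polls the signal for rising edges and calls Shoot, which draws energy from the grid manager and spawns BP_Projectile in a ShotCount-based pattern across five spawn points.
; At zero health it destroys its connected wire and itself, but only if that connection is valid.
; A head-turning function exists but is not called here.
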(event Custom|OnDamageRecieved_Event
  (bind _signalinput (Variables|Default|GetSignalInput))
  (bind _connectedoutput (Variables|/Game/TowerDefence/Blueprints/BPC_SignalInput.BPC_SignalInput_C|GetConnectedOutput _signalinput))
  (bind _returnvalue (Components|GetOwner _connectedoutput))
  (bind _health (CallFunction|GetHealth))
  (if (<= _health 0)
    (if (Utilities|IsValid _returnvalue)
      (bind _asbp_wire (Utilities|Casting|CastToBP_Wire _returnvalue))
      (Default|DestroyWire _asbp_wire)
      (Actor|DestroyActor))))

(event EventBeginPlay
  (EventDispatchers|AssignOnDamageRecieved (delegate Custom|OnDamageRecieved_Event)))

(event Collision|EventActorBeginOverlap
  (params (OtherActor :type Actor%20Object%20Reference)))

(event EventTick
  (params (DeltaSeconds :type Float%20%28single-precision%29))
  (bind _signalinput (Variables|Default|GetSignalInput))
  (bind _signal (Variables|/Game/TowerDefence/Blueprints/BPC_SignalInput.BPC_SignalInput_C|GetSignal _signalinput))
  (if (!= (Variables|Default|GetPreviousSignal) _signal)
    (if _signal
      (CallFunction|Shoot))
    (Variables|Default|SetPreviousSignal _signal)))

(fn ConstructionScript
  (bind _spawnlist (Variables|Shooting|GetSpawnList))
  (Utilities|Array|Add _spawnlist (Variables|Default|GetProjectileSpawnLocation0))
  (Utilities|Array|Add _spawnlist (Variables|Default|GetProjectileSpawnLocation1))
  (Utilities|Array|Add _spawnlist (Variables|Default|GetProjectileSpawnLocation2))
  (Utilities|Array|Add _spawnlist (Variables|Default|GetProjectileSpawnLocation3))
  (Utilities|Array|Add _spawnlist (Variables|Default|GetProjectileSpawnLocation4)))

(fn TurnHead
  (bind _turrethead (Variables|Default|GetTurretHead))
  (Transformation|AddRelativeRotation _turrethead (Math|Rotator|MakeRotator 0.0 0.0 (Variables|Shooting|GetTurretSpeed)) false false)
  (if (> 0.0 (.yaw (Variables|/Script/Engine.SceneComponent|GetRelativeRotation _turrethead)))
    (Variables|Shooting|SetTurretSpeed (* -1.0 (Variables|Shooting|GetTurretSpeed)))))

(fn SpawnArrowatPosition
  (params (index :type Integer))
  (Game|SpawnActorfromClass "/Game/TowerDefence/Blueprints/BP_Projectile.BP_Projectile_C" (Transformation|GetWorldTransform (Utilities|Array|Get(acopy) (Variables|Shooting|GetSpawnList) index)) "Undefined" "MultiplyWithRoot" 0 (Variables|Shooting|GetProjectileRange) 0))

(fn GetInputLocation
  (return (Transformation|GetWorldLocation (Variables|Default|GetSignalInput))))

(fn Shoot
  (bind _returnvalue (Actor|GetActorOfClass "/Game/TowerDefence/Blueprints/BP_GridManager.BP_GridManager_C"))
  (bind _consumed (Default|ConsumeEnergy _returnvalue (Variables|Default|GetEnergyCost)))
  (if _consumed
    (switch int (Variables|Shooting|GetShotCount)
      (:1
        (CallFunction|SpawnArrowatPosition 2))
      (:2
        (CallFunction|SpawnArrowatPosition 1)
        (CallFunction|SpawnArrowatPosition 3))
      (:3
        (CallFunction|SpawnArrowatPosition)
        (CallFunction|SpawnArrowatPosition 2)
        (CallFunction|SpawnArrowatPosition 4))
      (:4
        (CallFunction|SpawnArrowatPosition)
        (CallFunction|SpawnArrowatPosition 1)
        (CallFunction|SpawnArrowatPosition 2)
        (CallFunction|SpawnArrowatPosition 3))
      (:5
        (CallFunction|SpawnArrowatPosition)
        (CallFunction|SpawnArrowatPosition 1)
        (CallFunction|SpawnArrowatPosition 2)
        (CallFunction|SpawnArrowatPosition 3)
        (CallFunction|SpawnArrowatPosition 4)))))