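; Grid cell component for the tower defence game that holds a single placed actor.
; PlaceComponent spawns the given class at the cell's world location plus a placement offset, passing itself as parent cell, and returns whether the cell was free.
; ResetPlacedComponent clears the stored reference without destroying the actor.
; GetComponentSpawn only returns a zero vector, and BeginPlay and Tick are unused.
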(event EventBeginPlay)

(event EventTick
  (params (DeltaSeconds :type Float%20%28single-precision%29)))

(fn GetComponentSpawn
  (return "0, 0, 0"))

(fn PlaceComponent
  (params (ComponentClass :type BP%20Ally%20Building%20Class%20Reference) (Rotation :type Rotator))
  (bind _output_get (LocalVariables|SetIsValid (Utilities|IsValid (Variables|Default|GetPlacedActor))))
  (if _output_get
    _
    (else
      (bind _returnvalue (Game|SpawnActorfromClass ComponentClass (Math|Transform|MakeTransform (+ (Variables|Default|GetPlacementPosition) (Transformation|GetWorldLocation)) Rotation) "AlwaysSpawn" "MultiplyWithRoot" 0 self 0))
      (Variables|Default|SetPlacedActor _returnvalue)))
  (return (not (LocalVariables|GetIsValid))))

(fn ResetPlacedComponent
  (Variables|Default|SetPlacedActor 0))