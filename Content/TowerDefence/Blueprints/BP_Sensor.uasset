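; BP_Sensor is a tower defence actor that outputs a signal while an enemy is inside its scanning area.
; Each tick it checks the ScanningArea for overlapping BP_Enemy actors.
; It calls UpdateSignal on its SignalOutput component only when the detection state differs from the current signal.
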(event EventTick
  (params (DeltaSeconds :type Float%20%28single-precision%29))
  (bind _output_get (Variables|Default|SetEnemyDetected (> (Utilities|Array|Length (Collision|GetOverlappingActors (Variables|Default|GetScanningArea) "/Game/TowerDefence/Blueprints/BP_Enemy.BP_Enemy_C" :!class /Script/Engine.PrimitiveComponent)) 0)))
  (if (!= _output_get (Variables|/Game/TowerDefence/Blueprints/BPC_SignalOutput.BPC_SignalOutput_C|GetSignal (Variables|Default|GetSignal%20Output)))
    (Default|UpdateSignal (Variables|Default|GetSignal%20Output) (Variables|Default|GetEnemyDetected))))

(fn ConstructionScript)