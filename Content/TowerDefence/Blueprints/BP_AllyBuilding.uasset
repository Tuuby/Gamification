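; Player-side building actor for the tower defence game, with health, a health bar and grid placement.
; Damage lowers health and updates the bar widget, which turns to face the camera every tick.
; At zero health it destroys every wire on its signal input and output components, resets its grid cell, then destroys itself with a random deconstruction sound.
; A highlight function toggles custom depth on all its static meshes.
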(event EventTick
  (params (DeltaSeconds :type Float%20%28single-precision%29))
  (CallFunction|UpdateHealthBarRotation))

(event Game|Damage|EventAnyDamage
  (params (Damage :type Float%20%28single-precision%29) (DamageType :type Damage%20Type%20Object%20Reference) (InstigatedBy :type Controller%20Object%20Reference) (DamageCauser :type Actor%20Object%20Reference))
  (CallFunction|ReduceHealth Damage)
  (CallFunction|UpdateHealthBar)
  (if (<= (Variables|Default|GetHealthPoints) 0.0)
    (CallFunction|DestroySelf)))

(fn ConstructionScript)

(fn DestroySelf
  ;[0.05127 0.05127 0.05127] Get and destroy the wire connected to all Inputs
  (for _array_element (Actor|GetComponentsByClass "/Game/TowerDefence/Blueprints/BPC_SignalInput.BPC_SignalInput_C")
    (Utilities|IsValid (Variables|/Game/TowerDefence/Blueprints/BPC_SignalInput.BPC_SignalInput_C|GetConnectedOutput _array_element)
      (:Is%20Valid
        (Utilities|IsValid (Components|GetOwner (Variables|/Game/TowerDefence/Blueprints/BPC_SignalInput.BPC_SignalInput_C|GetConnectedOutput _array_element))
          (:Is%20Valid
            (bind _asbp_wire (Utilities|Casting|CastToBP_Wire (Components|GetOwner (Variables|/Game/TowerDefence/Blueprints/BPC_SignalInput.BPC_SignalInput_C|GetConnectedOutput _array_element))))
            (Default|DestroyWire _asbp_wire))))))
  ;[0.05127 0.05127 0.05127] Get and destroy all wires connected to all Outputs
  (for _array_element_2 (Actor|GetComponentsByClass "/Game/TowerDefence/Blueprints/BPC_SignalOutput.BPC_SignalOutput_C")
    (for _array_element_3 (Variables|/Game/TowerDefence/Blueprints/BPC_SignalOutput.BPC_SignalOutput_C|GetConnections _array_element_2)
      (Utilities|IsValid (Components|GetOwner _array_element_3)
        (:Is%20Valid
          (bind _asbp_wire_2 (Utilities|Casting|CastToBP_Wire (Components|GetOwner _array_element_3)))
          (Default|DestroyWire _asbp_wire_2)))))
  ;[0.05127 0.05127 0.05127] Notify GridCell and Destroy self
  (Default|ResetPlacedComponent (Variables|Default|GetParentGridcell) self)
  (Actor|DestroyActor)
  (CallFunction|PlayDeconstructionSound))

(fn ReduceHealth
  (params (InputPin :type Float%20%28single-precision%29))
  (Variables|Default|SetHealthPoints (- (Variables|Default|GetHealthPoints) InputPin))
  (return))

(fn HighlightBuilding
  (params (Enabled :type Boolean))
  (for _array_element (Actor|GetComponentsByClass "/Script/Engine.StaticMeshComponent")
    (Rendering|SetRenderCustomDepth _array_element Enabled)))

(fn PlayDeconstructionSound
  (Audio|PlaySound2D (.OutItem (Utilities|Array|Random (Variables|Default|GetDeconstructionSounds))) 1.0 1.0 0.0 0 0))

(fn UpdateHealthBar
  (bind _aswidget_ally_healthbar (Utilities|Casting|CastToWidget_AllyHealthbar (UserInterface|GetWidget (Variables|Default|GetHealth%20Bar%20Widget))))
  (bind _output_get (Variables|Default|SetPercent (/ (Variables|Default|GetHealthPoints) (Variables|Default|GetMaxHealth))))
  (Progress|SetPercent (Variables|/Game/TowerDefence/UI/Widget_AllyHealthbar.Widget_AllyHealthbar_C|GetHealthBar _aswidget_ally_healthbar) _output_get))

(fn UpdateHealthBarRotation
  (bind _health_bar_widget (Variables|Default|GetHealth%20Bar%20Widget))
  (Utilities|IsValid _health_bar_widget
    (:Is%20Valid
      (Transformation|SetWorldRotation _health_bar_widget (Math|Rotator|FindLookatRotation (Transformation|GetWorldLocation _health_bar_widget) (Transformation|GetWorldLocation (Variables|/Script/Engine.PlayerCameraManager|GetTransformComponent (Game|GetPlayerCameraManager 0)))) false false))))