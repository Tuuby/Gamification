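; Actor component that acts as a clock generator, producing a square-wave signal for the tower defence signal system.
; On BeginPlay it caches the owner's BPC_SignalOutput component.
; Each tick it accumulates time and flips that output's signal every half period of the configured Frequency, resetting the timer to zero on each toggle.
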(event EventBeginPlay
  (bind _returnvalue (Components|GetOwner))
  (bind _returnvalue_2 (Actor|GetComponentbyClass _returnvalue "/Game/TowerDefence/Blueprints/BPC_SignalOutput.BPC_SignalOutput_C"))
  (Utilities|IsValid _returnvalue_2
    (:Is%20Valid
      (Variables|Default|SetSingalOutput _returnvalue_2))))

(event EventTick
  (params (DeltaSeconds :type Float%20%28single-precision%29))
  (CallFunction|CheckClock DeltaSeconds))

(fn CheckClock
  (params (DeltaSeconds :type Float%20%28double-precision%29))
  (bind _output_get (Variables|Default|SetTimeSinceLast (+ DeltaSeconds (Variables|Default|GetTimeSinceLast))))
  (if (> _output_get (/ 1.0 (* (Variables|Default|GetFrequency) 2.0)))
    (Default|UpdateSignal (Variables|Default|GetSingalOutput) (not (Variables|/Game/TowerDefence/Blueprints/BPC_SignalOutput.BPC_SignalOutput_C|GetSignal (Variables|Default|GetSingalOutput))))
    (Variables|Default|SetTimeSinceLast 0.0)))