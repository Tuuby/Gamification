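; Tower defence connector actor that relays a boolean signal through a placed network.
; SetSignal stores the value, forwards it to every entry in Connections with no change or cycle check, then calls SetMaterial based on the state.
; SetMaterial applies the given material to the X and Y cylinders, repeating both assignments.
; The construction script snaps the root to a 100-unit world grid.
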(event EventBeginPlay)

(event Collision|EventActorBeginOverlap
  (params (OtherActor :type Actor%20Object%20Reference)))

(event EventTick
  (params (DeltaSeconds :type Float%20%28single-precision%29)))

(event EventSetSignal
  (params (Signal :type Boolean))
  (bind _output_get (Variables|Default|SetSignal Signal))
  (for _array_element (Variables|Default|GetConnections)
    (Default|SetSignal _array_element _output_get))
  (if (Variables|Default|GetSignal)
    (CallFunction|SetMaterial)
    (else
      (CallFunction|SetMaterial))))

(fn ConstructionScript
  (Transformation|SetWorldLocation (Variables|Default|GetDefaultSceneRoot) (Class|KismetMathLibrary|VectorSnappedtoGrid (Transformation|GetActorLocation) 1e+02) false false))

(fn SetMaterial
  (params (TargetMaterial :type Material%20Object%20Reference))
  (Utilities|FlowControl|Sequence
    (:then_0
      (Rendering|Material|SetMaterial (Variables|Default|GetCylinderX) 0 TargetMaterial))
    (:then_1
      (Rendering|Material|SetMaterial (Variables|Default|GetCylinderY) 0 TargetMaterial))
    (:then_2
      (Rendering|Material|SetMaterial (Variables|Default|GetCylinder-X) 0 TargetMaterial))
    (:then_3
      (Rendering|Material|SetMaterial (Variables|Default|GetCylinder-Y) 0 TargetMaterial))))