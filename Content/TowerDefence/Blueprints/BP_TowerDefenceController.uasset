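; Player controller for the tower defence game, handling camera, building, wiring and bulldozing on the grid.
; Enhanced Input drives a bounded pan, zoom and rotate camera pawn that can flip upside down.
; Each tick, a cursor trace feeds tool-specific highlighting via custom depth or target calls, with post-process materials swapped per tool.
; Clicks place components or output-to-input wires through GridManager, or destroy highlighted buildings and wires; slot keys drive the UI.
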(event Input|EnhancedActionEvents|EnhancedInputActionIA_SetCameraX
  (params (ActionValue :type Float%20%28double-precision%29) (ElapsedSeconds :type Float%20%28double-precision%29) (TriggeredSeconds :type Float%20%28double-precision%29) (InputAction :type Input%20Action%20Object%20Reference :default "/Game/TowerDefence/Input/Actions/IA_SetCameraX.IA_SetCameraX"))
  ;[0.05098 0.05098 0.05098] Camera Movement
  (:Triggered
    (Variables|Camera|SetMovementDirection (+ (Variables|Camera|GetMovementDirection) (Math|Vector|MakeVector ActionValue 0.0 0.0))))
  (:Completed
    (Variables|Camera|SetMovementDirection (* (Variables|Camera|GetMovementDirection) "0.000000,1.000000,1.000000"))))

(event Input|EnhancedActionEvents|EnhancedInputActionIA_SetCameraY
  (params (ActionValue :type Float%20%28double-precision%29) (ElapsedSeconds :type Float%20%28double-precision%29) (TriggeredSeconds :type Float%20%28double-precision%29) (InputAction :type Input%20Action%20Object%20Reference :default "/Game/TowerDefence/Input/Actions/IA_SetCameraY.IA_SetCameraY"))
  ;[0.05098 0.05098 0.05098] Camera Movement
  (:Triggered
    (Variables|Camera|SetMovementDirection (+ (Variables|Camera|GetMovementDirection) (Math|Vector|MakeVector 0.0 ActionValue 0.0))))
  (:Completed
    (Variables|Camera|SetMovementDirection (* (Variables|Camera|GetMovementDirection) "1.000000,0.000000,1.000000"))))

(event Input|EnhancedActionEvents|EnhancedInputActionIA_SelectSlot2
  (params (ActionValue :type Boolean) (ElapsedSeconds :type Float%20%28double-precision%29) (TriggeredSeconds :type Float%20%28double-precision%29) (InputAction :type Input%20Action%20Object%20Reference :default "/Game/TowerDefence/Input/Actions/IA_SelectSlot2.IA_SelectSlot2"))
  (bind _ui (Variables|Default|GetUI))
  (bind _wiretoolenabled (Variables|WireTool|GetWiretoolEnabled))
  ;[0.05127 0.05127 0.05127] Select Components to Build
  (if (Class|Widget|GetIsEnabled (Variables|/Game/TowerDefence/UI/Widget_UserInterface.Widget_UserInterface_C|GetSlot2Button _ui))
    (if _wiretoolenabled
      (WireTool|ToggleWireTool _wiretoolenabled))
    (Default|ToggleButtonState _ui 1)))

(event Input|EnhancedActionEvents|EnhancedInputActionIA_SelectSlot3
  (params (ActionValue :type Boolean) (ElapsedSeconds :type Float%20%28double-precision%29) (TriggeredSeconds :type Float%20%28double-precision%29) (InputAction :type Input%20Action%20Object%20Reference :default "/Game/TowerDefence/Input/Actions/IA_SelectSlot3.IA_SelectSlot3"))
  (bind _ui (Variables|Default|GetUI))
  (bind _wiretoolenabled (Variables|WireTool|GetWiretoolEnabled))
  ;[0.05127 0.05127 0.05127] Select Components to Build
  (if (Class|Widget|GetIsEnabled (Variables|/Game/TowerDefence/UI/Widget_UserInterface.Widget_UserInterface_C|GetSlot3Button _ui))
    (if _wiretoolenabled
      (WireTool|ToggleWireTool _wiretoolenabled))
    (Default|ToggleButtonState _ui 2)))

(event Input|EnhancedActionEvents|EnhancedInputActionIA_SelectSlot4
  (params (ActionValue :type Boolean) (ElapsedSeconds :type Float%20%28double-precision%29) (TriggeredSeconds :type Float%20%28double-precision%29) (InputAction :type Input%20Action%20Object%20Reference :default "/Game/TowerDefence/Input/Actions/IA_SelectSlot4.IA_SelectSlot4"))
  (bind _ui (Variables|Default|GetUI))
  (bind _wiretoolenabled (Variables|WireTool|GetWiretoolEnabled))
  ;[0.05127 0.05127 0.05127] Select Components to Build
  (if (Class|Widget|GetIsEnabled (Variables|/Game/TowerDefence/UI/Widget_UserInterface.Widget_UserInterface_C|GetSlot4Button _ui))
    (if _wiretoolenabled
      (WireTool|ToggleWireTool _wiretoolenabled))
    (Default|ToggleButtonState _ui 3)))

(event Input|EnhancedActionEvents|EnhancedInputActionIA_BulldozerToggle
  (params (ActionValue :type Boolean) (ElapsedSeconds :type Float%20%28double-precision%29) (TriggeredSeconds :type Float%20%28double-precision%29) (InputAction :type Input%20Action%20Object%20Reference :default "/Game/TowerDefence/Input/Actions/IA_BulldozerToggle.IA_BulldozerToggle"))
  (Bulldozer|ToggleBulldozer (Variables|Bulldozer|GetBulldozerEnabled)))

(event Input|EnhancedActionEvents|EnhancedInputActionIA_Zoom
  (params (ActionValue :type Float%20%28double-precision%29) (ElapsedSeconds :type Float%20%28double-precision%29) (TriggeredSeconds :type Float%20%28double-precision%29) (InputAction :type Input%20Action%20Object%20Reference :default "/Game/TowerDefence/Input/Actions/IA_Zoom.IA_Zoom"))
  ;[0.05098 0.05098 0.05098] Camera Zoom
  (Variables|Camera|SetCameraZoom (Math|Float|Clamp(Float) (+ (* ActionValue -0.05) (Variables|Camera|GetCameraZoom)))))

(event Input|EnhancedActionEvents|EnhancedInputActionIA_CameraRotation
  (params (ActionValue :type Float%20%28double-precision%29) (ElapsedSeconds :type Float%20%28double-precision%29) (TriggeredSeconds :type Float%20%28double-precision%29) (InputAction :type Input%20Action%20Object%20Reference :default "/Game/TowerDefence/Input/Actions/IA_CameraRotation.IA_CameraRotation"))
  ;[0.05127 0.05127 0.05127] Camera Rotation
  (if (Variables|Camera|GetUpsideDown)
    (Variables|Camera|SetCameraRotationInput (* ActionValue -1.0))
    (else
      (Variables|Camera|SetCameraRotationInput ActionValue)))
  (Variables|Camera|SetCameraRotation (+ (* (Variables|Camera|GetCameraRotationInput) 1.0) (Variables|Camera|GetCameraRotation))))

(event Input|EnhancedActionEvents|EnhancedInputActionIA_PlaceComponent
  (params (ActionValue :type Boolean) (ElapsedSeconds :type Float%20%28double-precision%29) (TriggeredSeconds :type Float%20%28double-precision%29) (InputAction :type Input%20Action%20Object%20Reference :default "/Game/TowerDefence/Input/Actions/IA_PlaceComponent.IA_PlaceComponent"))
  (bind _gridmanager (Variables|Grid|GetGridManager))
  (bind _highlightedtile (Variables|Highlighting|GetHighlightedTile))
  ;[0.05127 0.05127 0.05127] Component & Wire Building
  (if (Variables|/Game/TowerDefence/Blueprints/BP_GridManager.BP_GridManager_C|GetDialogShowing _gridmanager)
    (Default|RemoveDialogWidget _gridmanager)
    (elif (Variables|WireTool|GetWiretoolEnabled)
      (WireTool|SelectWirePoints)
      (elif (Variables|Bulldozer|GetBulldozerEnabled)
        (Bulldozer|DeconstructObject)
        (elif (Utilities|IsValid _highlightedtile)
          (Default|PlaceComponent (Variables|Grid|GetGridManager) _highlightedtile))))))

(event Input|EnhancedActionEvents|EnhancedInputActionIA_SelectSlot1
  (params (ActionValue :type Boolean) (ElapsedSeconds :type Float%20%28double-precision%29) (TriggeredSeconds :type Float%20%28double-precision%29) (InputAction :type Input%20Action%20Object%20Reference :default "/Game/TowerDefence/Input/Actions/IA_SelectSlot1.IA_SelectSlot1"))
  (bind _ui (Variables|Default|GetUI))
  (bind _wiretoolenabled (Variables|WireTool|GetWiretoolEnabled))
  ;[0.05127 0.05127 0.05127] Select Components to Build
  (if (Class|Widget|GetIsEnabled (Variables|/Game/TowerDefence/UI/Widget_UserInterface.Widget_UserInterface_C|GetSlot1Button _ui))
    (if _wiretoolenabled
      (WireTool|ToggleWireTool _wiretoolenabled))
    (Default|ToggleButtonState _ui)))

(event Input|EnhancedActionEvents|EnhancedInputActionIA_RotateBuilding
  (params (ActionValue :type Boolean) (ElapsedSeconds :type Float%20%28double-precision%29) (TriggeredSeconds :type Float%20%28double-precision%29) (InputAction :type Input%20Action%20Object%20Reference :default "/Game/TowerDefence/Input/Actions/IA_RotateBuilding.IA_RotateBuilding"))
  ;[0.05127 0.05127 0.05127] Rotate Component to Build
  (Default|RotateComponent (Variables|Grid|GetGridManager)))

(event Input|EnhancedActionEvents|EnhancedInputActionIA_SwitchView
  (params (ActionValue :type Boolean) (ElapsedSeconds :type Float%20%28double-precision%29) (TriggeredSeconds :type Float%20%28double-precision%29) (InputAction :type Input%20Action%20Object%20Reference :default "/Game/TowerDefence/Input/Actions/IA_SwitchView.IA_SwitchView"))
  ;[0.05127 0.05127 0.05127] Switch view of the grid
  (Camera|SwitchView))

(event Input|EnhancedActionEvents|EnhancedInputActionIA_ToggleWireTool
  (params (ActionValue :type Boolean) (ElapsedSeconds :type Float%20%28double-precision%29) (TriggeredSeconds :type Float%20%28double-precision%29) (InputAction :type Input%20Action%20Object%20Reference :default "/Game/TowerDefence/Input/Actions/IA_ToggleWireTool.IA_ToggleWireTool"))
  ;[0.05127 0.05127 0.05127] Toggle Wire Tool
  (WireTool|ToggleWireTool (Variables|WireTool|GetWiretoolEnabled)))

(event Input|EnhancedActionEvents|EnhancedInputActionIA_PauseGame
  (params (ActionValue :type Boolean) (ElapsedSeconds :type Float%20%28double-precision%29) (TriggeredSeconds :type Float%20%28double-precision%29) (InputAction :type Input%20Action%20Object%20Reference :default "/Game/TowerDefence/Input/Actions/IA_PauseGame.IA_PauseGame"))
  ;[0.05127 0.05127 0.05127] Pause Game
  (if (Game|IsGamePaused)
    (Game|SetGamePaused false)
    (else
      (Game|SetGamePaused true))))

(event EventBeginPlay
  (bind _returnvalue (PlayerController|LocalPlayerSubsystems|GetEnhancedInputLocalPlayerSubsystem))
  ;[0.05127 0.05127 0.05127] Add Mapping Context & Initialize the CameraPawn
  (Utilities|IsValid _returnvalue
    (:Is%20Valid
      (Input|AddMappingContext _returnvalue "/Game/TowerDefence/Input/IMC_Default.IMC_Default" 0 "(bIgnoreAllPressedKeysUntilRelease=True,bForceImmediately=False,bNotifyUserSettings=False)")
      (Variables|Camera|SetCameraPawn (Pawn|GetControlledPawn))
      (Input|SetInputModeGameandUI self 0 "LockAlways" false false)
      ;[0.05127 0.05127 0.05127] Get Total Grid size
      (bind _returnvalue_2 (Actor|GetActorOfClass "/Game/TowerDefence/Blueprints/BP_GridManager.BP_GridManager_C"))
      (Variables|Grid|SetGridManager _returnvalue_2)
      (Variables|Grid|SetTotalGridSize (* (Variables|/Game/TowerDefence/Blueprints/BP_GridManager.BP_GridManager_C|GetGridSizeX _returnvalue_2) (Variables|/Game/TowerDefence/Blueprints/BP_GridManager.BP_GridManager_C|GetGridSpacing _returnvalue_2)))
      ;[0.05127 0.05127 0.05127] Get a reference to the UI
      (bind _foundwidgets (Widget|GetAllWidgetsOfClass "/Game/TowerDefence/UI/Widget_UserInterface.Widget_UserInterface_C" true))
      (Variables|Default|SetUI (Utilities|Array|Get(acopy) _foundwidgets))
      ;[0.05127 0.05127 0.05127] Get reference to PostProcessVolume
      (bind _returnvalue_3 (Actor|GetActorOfClass "/Script/Engine.PostProcessVolume"))
      (Variables|Default|SetHighlightPostProcesser _returnvalue_3)
      (Highlighting|ChoosePostProcessMaterial))))

(event EventTick
  (params (DeltaSeconds :type Float%20%28single-precision%29))
  ;[0.05127 0.05127 0.05127] Game Tick
  (Camera|MoveCamera)
  (Highlighting|GetMouseTargets)
  (if (Variables|WireTool|GetWiretoolEnabled)
    (Highlighting|HighlightInput)
    (Highlighting|HighlightOutput)
    (elif (Variables|Bulldozer|GetBulldozerEnabled)
      (Highlighting|HighlightAllyBuilding)
      (Highlighting|HighlightWire)
      (else
        (Highlighting|HighlightTile)))))

(fn ConstructionScript)

(fn MoveCamera
  (bind _movementdirection (Variables|Camera|GetMovementDirection))
  (bind _mincameraspeed (Variables|Camera|GetMinCameraSpeed))
  (bind _camerazoom (Variables|Camera|GetCameraZoom))
  (bind _maxcameraspeed (Variables|Camera|GetMaxCameraSpeed))
  (bind _camerapawn (Variables|Camera|GetCameraPawn))
  (bind _camerapawn_2 (Variables|Camera|GetCameraPawn))
  (bind _totalgridsize (Variables|Grid|GetTotalGridSize))
  (bind _returnvalue (Math|Float|Lerp _mincameraspeed _maxcameraspeed _camerazoom))
  (bind _returnvalue_2 (Transformation|GetActorLocation _camerapawn))
  (bind _returnvalue_3 (Transformation|GetActorRotation _camerapawn_2))
  (bind _returnvalue_4 (/ _totalgridsize 2.0))
  (bind _returnvalue_5 (Math|Vector|RotateVector _movementdirection _returnvalue_3))
  (bind _returnvalue_6 (* _returnvalue_4 -1.0))
  (bind _returnvalue_7 (Math|Vector|Normalize _returnvalue_5))
  (bind _returnvalue_8 (* _returnvalue_7 _returnvalue))
  (bind _returnvalue_9 (+ _returnvalue_2 _returnvalue_8))
  (if (Variables|Camera|GetUpsideDown)
    (LocalVariables|SetRollAngle 1.8e+02)
    (else
      (LocalVariables|SetRollAngle 0.0)))
  (bind _returnvalue_10 (Class|WidgetLayoutLibrary|GetMousePositiononViewport))
  (Variables|Camera|SetMouseX (.x _returnvalue_10))
  (Variables|Camera|SetMouseY (.y _returnvalue_10))
  (Transformation|SetActorLocationAndRotation _camerapawn (Math|Vector|MakeVector (Math|Float|Clamp(Float) (.x _returnvalue_9) _returnvalue_6 _returnvalue_4) (Math|Float|Clamp(Float) (.y _returnvalue_9) _returnvalue_6 _returnvalue_4) 0.0) (Math|Rotator|MakeRotator (LocalVariables|GetRollAngle) 0.0 (Variables|Camera|GetCameraRotation)))
  (bind _asbp_camera_pawn (Utilities|Casting|CastToBP_CameraPawn (Variables|Camera|GetCameraPawn)))
  (Variables|/Script/Engine.SpringArmComponent|SetTargetArmLength (Variables|/Game/TowerDefence/Blueprints/BP_CameraPawn.BP_CameraPawn_C|GetSpringArm _asbp_camera_pawn) (Math|Float|Lerp (Variables|Camera|GetMinZoomDistance) (Variables|Camera|GetMaxZoomDistance) (Variables|Camera|GetCameraZoom))))

(fn HighlightTile
  (bind _asbp_grid_cell (Utilities|Casting|CastToBP_GridCell (Variables|Highlighting|GetTargetedActor))
    (:then
      (LocalVariables|SetTargetedGridCell _asbp_grid_cell)
      (if (and (Utilities|IsValid (Variables|Highlighting|GetHighlightedTile)) (!= _asbp_grid_cell (Variables|Highlighting|GetHighlightedTile)))
        (Rendering|SetRenderCustomDepth (Variables|/Game/TowerDefence/Blueprints/BP_GridCell.BP_GridCell_C|GetTile (Variables|Highlighting|GetHighlightedTile)) false))
      (bind _output_get (Variables|Highlighting|SetHighlightedTile (LocalVariables|GetTargetedGridCell)))
      (Rendering|SetRenderCustomDepth (Variables|/Game/TowerDefence/Blueprints/BP_GridCell.BP_GridCell_C|GetTile _output_get) true))
    (:CastFailed
      (if (Utilities|IsValid (Variables|Highlighting|GetHighlightedTile))
        (Rendering|SetRenderCustomDepth (Variables|/Game/TowerDefence/Blueprints/BP_GridCell.BP_GridCell_C|GetTile (Variables|Highlighting|GetHighlightedTile)) false)
        (Variables|Highlighting|SetHighlightedTile 0)))))

(fn SwitchView
  (Variables|Camera|SetUpsideDown (not (Variables|Camera|GetUpsideDown))))

(fn GetMouseTargets
  (bind _array (Utilities|Array|MakeArray "ObjectTypeQuery2"))
  (bind (_hitresult _returnvalue) (Class|PlayerController|GetHitResultUnderCursorforObjects _array true))
  (bind (_bblockinghit _binitialoverlap _time _distance _location _impactpoint _normal _impactnormal _physmat _hitactor _hitcomponent) (Collision|BreakHitResult _hitresult))
  (if _returnvalue
    (Variables|Highlighting|SetTargetedActor _hitactor)
    (Variables|Highlighting|SetTargetedComponent _hitcomponent)
    (else
      (Variables|Highlighting|SetTargetedActor 0)
      (Variables|Highlighting|SetTargetedComponent 0))))

(fn ChoosePostProcessMaterial
  (params (Index :type Integer))
  (switch int Index
    (:Default
      (bind _returnvalue (Rendering|Material|CreateDynamicMaterialInstance "/Game/TowerDefence/Materials/M_Highlights.M_Highlights" "None" "None" :!class /Script/Engine.KismetMaterialLibrary))
      (Rendering|AddorUpdateBlendable (Variables|Default|GetHighlightPostProcesser) _returnvalue 1.0 :!class /Script/Engine.PostProcessVolume))
    (:0
      (bind _returnvalue_2 (Rendering|Material|CreateDynamicMaterialInstance "/Game/TowerDefence/Materials/MI_TileHighlight.MI_TileHighlight" "None" "None" :!class /Script/Engine.KismetMaterialLibrary))
      (Rendering|AddorUpdateBlendable (Variables|Default|GetHighlightPostProcesser) _returnvalue_2 1.0 :!class /Script/Engine.PostProcessVolume))
    (:1
      (bind _returnvalue_3 (Rendering|Material|CreateDynamicMaterialInstance "/Game/TowerDefence/Materials/MI_InOutHighlight.MI_InOutHighlight" "None" "None" :!class /Script/Engine.KismetMaterialLibrary))
      (Rendering|AddorUpdateBlendable (Variables|Default|GetHighlightPostProcesser) _returnvalue_3 1.0 :!class /Script/Engine.PostProcessVolume))
    (:2
      (bind _returnvalue_4 (Rendering|Material|CreateDynamicMaterialInstance "/Game/TowerDefence/Materials/MI_BulldozerHighlight.MI_BulldozerHighlight" "None" "None" :!class /Script/Engine.KismetMaterialLibrary))
      (Rendering|AddorUpdateBlendable (Variables|Default|GetHighlightPostProcesser) _returnvalue_4 1.0 :!class /Script/Engine.PostProcessVolume))))

(fn HighlightInput
  (bind _asbpc_signal_input (Utilities|Casting|CastToBPC_SignalInput (Variables|Highlighting|GetTargetedComponent))
    (:then
      (LocalVariables|SetTargetedInput _asbpc_signal_input)
      (if (and (Utilities|IsValid (Variables|Highlighting|GetHighlightedInput)) (!= _asbpc_signal_input (Variables|Highlighting|GetHighlightedInput)))
        (Rendering|SetRenderCustomDepth (Variables|Highlighting|GetHighlightedInput) false))
      (bind _output_get (Variables|Highlighting|SetHighlightedInput (LocalVariables|GetTargetedInput)))
      (Rendering|SetRenderCustomDepth _output_get true))
    (:CastFailed
      (if (Utilities|IsValid (Variables|Highlighting|GetHighlightedInput))
        (Rendering|SetRenderCustomDepth (Variables|Highlighting|GetHighlightedInput) false)
        (Variables|Highlighting|SetHighlightedInput 0)))))

(fn HighlightOutput
  (bind _asbpc_signal_output (Utilities|Casting|CastToBPC_SignalOutput (Variables|Highlighting|GetTargetedComponent))
    (:then
      (LocalVariables|SetTargetedOutput _asbpc_signal_output)
      (if (and (Utilities|IsValid (Variables|Highlighting|GetHighlightedOutput)) (!= _asbpc_signal_output (Variables|Highlighting|GetHighlightedOutput)))
        (Rendering|SetRenderCustomDepth (Variables|Highlighting|GetHighlightedOutput) false))
      (bind _output_get (Variables|Highlighting|SetHighlightedOutput (LocalVariables|GetTargetedOutput)))
      (Rendering|SetRenderCustomDepth _output_get true))
    (:CastFailed
      (if (Utilities|IsValid (Variables|Highlighting|GetHighlightedOutput))
        (Rendering|SetRenderCustomDepth (Variables|Highlighting|GetHighlightedOutput) false)
        (Variables|Highlighting|SetHighlightedOutput 0)))))

(fn ToggleWireTool
  (params (PreviousState :type Boolean))
  (bind _output_get (Variables|WireTool|SetWiretoolEnabled (not PreviousState)))
  (if _output_get
    (Highlighting|ChoosePostProcessMaterial 1)
    (else
      (Highlighting|ChoosePostProcessMaterial)))
  (CallFunction|ResetSelectedComponent)
  (Highlighting|ResetHighlights))

(fn ResetHighlights
  (Utilities|FlowControl|Sequence
    (:then_0
      (Utilities|IsValid (Variables|Highlighting|GetHighlightedTile)
        (:Is%20Valid
          (Rendering|SetRenderCustomDepth (Variables|/Game/TowerDefence/Blueprints/BP_GridCell.BP_GridCell_C|GetTile (Variables|Highlighting|GetHighlightedTile)) false)
          (Variables|Highlighting|SetHighlightedTile 0))))
    (:then_1
      (Utilities|IsValid (Variables|Highlighting|GetHighlightedInput)
        (:Is%20Valid
          (Rendering|SetRenderCustomDepth (Variables|Highlighting|GetHighlightedInput) false)
          (Variables|Highlighting|SetHighlightedInput 0))))
    (:then_2
      (Utilities|IsValid (Variables|Highlighting|GetHighlightedOutput)
        (:Is%20Valid
          (Rendering|SetRenderCustomDepth (Variables|Highlighting|GetHighlightedOutput) false)
          (Variables|Highlighting|SetHighlightedOutput 0))))))

(fn ResetSelectedComponent
  (bind _gridmanager (Variables|Grid|GetGridManager))
  (bind _activeindex (Variables|/Game/TowerDefence/Blueprints/BP_GridManager.BP_GridManager_C|GetActiveIndex _gridmanager))
  (if (>= _activeindex 0)
    (Default|SetButtonState (Variables|Default|GetUI) _activeindex false)
    (Default|ResetComponent _gridmanager)))

(fn ToggleBulldozer
  (params (PreviousState :type Boolean))
  (bind _wiretoolenabled (Variables|WireTool|GetWiretoolEnabled))
  (if _wiretoolenabled
    (WireTool|ToggleWireTool _wiretoolenabled))
  (bind _output_get (Variables|Bulldozer|SetBulldozerEnabled (not PreviousState)))
  (if _output_get
    (Highlighting|ChoosePostProcessMaterial 2)
    (else
      (Highlighting|ChoosePostProcessMaterial)))
  (CallFunction|ResetSelectedComponent)
  (Highlighting|ResetHighlights))

(fn HighlightAllyBuilding
  (bind _asbp_ally_building (Utilities|Casting|CastToBP_AllyBuilding (Variables|Highlighting|GetTargetedActor))
    (:then
      (LocalVariables|SetTargetedAllyBuilding _asbp_ally_building)
      (if (and (Utilities|IsValid (Variables|Highlighting|GetHighlightedAllyBuilding)) (!= _asbp_ally_building (Variables|Highlighting|GetHighlightedAllyBuilding)))
        (Default|HighlightBuilding (Variables|Highlighting|GetHighlightedAllyBuilding) false))
      (bind _output_get (Variables|Highlighting|SetHighlightedAllyBuilding (LocalVariables|GetTargetedAllyBuilding)))
      (Default|HighlightBuilding _output_get true))
    (:CastFailed
      (if (Utilities|IsValid (Variables|Highlighting|GetHighlightedAllyBuilding))
        (Default|HighlightBuilding (Variables|Highlighting|GetHighlightedAllyBuilding) false)
        (Variables|Highlighting|SetHighlightedAllyBuilding 0)))))

(fn HighlightWire
  (bind _asbp_wire (Utilities|Casting|CastToBP_Wire (Variables|Highlighting|GetTargetedActor))
    (:then
      (LocalVariables|SetTargetedWire _asbp_wire)
      (if (and (Utilities|IsValid (Variables|Highlighting|GetHighlightedWire)) (!= _asbp_wire (Variables|Highlighting|GetHighlightedWire)))
        (Default|HighlightWire (Variables|Highlighting|GetHighlightedWire) false))
      (bind _output_get (Variables|Highlighting|SetHighlightedWire (LocalVariables|GetTargetedWire)))
      (Default|HighlightWire _output_get true))
    (:CastFailed
      (if (Utilities|IsValid (Variables|Highlighting|GetHighlightedWire))
        (Default|HighlightWire (Variables|Highlighting|GetHighlightedWire) false)
        (Variables|Highlighting|SetHighlightedWire 0)))))

(fn SelectWirePoints
  (bind _array (Utilities|Array|MakeArray "ObjectTypeQuery2"))
  (bind _hitresult (Class|PlayerController|GetHitResultUnderCursorforObjects _array true))
  (bind _hitcomponent (Collision|BreakHitResult _hitresult))
  (if (Variables|WireTool|GetInProgress)
    (bind _asbpc_signal_input (Utilities|Casting|CastToBPC_SignalInput _hitcomponent))
    (bind _output_get (Variables|WireTool|SetSignalDestination _asbpc_signal_input))
    (Default|PlaceWire (Variables|Grid|GetGridManager) (Variables|WireTool|GetSignalSource) _output_get)
    (Variables|WireTool|SetSignalSource 0)
    (Variables|WireTool|SetSignalDestination 0)
    (Variables|WireTool|SetInProgress false)
    (else
      (bind _asbpc_signal_output (Utilities|Casting|CastToBPC_SignalOutput _hitcomponent))
      (Variables|WireTool|SetSignalSource _asbpc_signal_output)
      (Variables|WireTool|SetInProgress true))))

(fn DeconstructObject
  (bind _highlightedwire (Variables|Highlighting|GetHighlightedWire))
  (bind _highlightedallybuilding (Variables|Highlighting|GetHighlightedAllyBuilding))
  (bind _returnvalue (Utilities|IsValid _highlightedallybuilding))
  (bind _returnvalue_2 (Utilities|IsValid _highlightedwire))
  (bind _returnvalue_3 (Class|KismetMathLibrary|XORBoolean _returnvalue _returnvalue_2))
  (if (and _returnvalue_3 _returnvalue)
    (Default|DestroySelf _highlightedallybuilding)
    (elif (and _returnvalue_3 _returnvalue_2)
      (Default|DestroyWire _highlightedwire))))

(fn SwitchTool
  (params (ToolID :type Integer))
  (switch int ToolID))