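; BP_GridManager is a tower defence actor that builds a square grid of BP_GridCell actors when play begins.
; MakeGrid offsets the start corner from the manager's location by half of GridSize times GridSpacing on X and Y.
; Nested loops spawn cells at GridSpacing intervals, ignoring collisions, and store each one in the GridCells array.
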(event EventBeginPlay
  (CallFunction|MakeGrid))

(event Collision|EventActorBeginOverlap
  (params (OtherActor :type Actor%20Object%20Reference)))

(event EventTick
  (params (DeltaSeconds :type Float%20%28single-precision%29)))

(fn ConstructionScript)

(fn MakeGrid
  (bind _returnvalue (Transformation|GetActorLocation))
  (bind _gridsize (Variables|Default|GetGridSize))
  (bind _gridspacing (Variables|Default|GetGridSpacing))
  (bind _returnvalue_2 (* _gridsize _gridspacing))
  (bind _returnvalue_3 (/ _returnvalue_2 2.0))
  (LocalVariables|SetStartingLocation (Math|Vector|MakeVector (- (.x _returnvalue) _returnvalue_3) (- (.y _returnvalue) _returnvalue_3) (.z _returnvalue)))
  (for _index (range 0 (Variables|Default|GetGridSize))
    (for _index_2 (range 0 (Variables|Default|GetGridSize))
      (Game|SpawnActorfromClass "/Game/TowerDefence/Blueprints/BP_GridCell.BP_GridCell_C" (Math|Transform|MakeTransform (+ (Math|Vector|MakeVector (Math|Conversions|ToFloat(Integer) (* _index_2 (Variables|Default|GetGridSpacing))) (Math|Conversions|ToFloat(Integer) (* _index (Variables|Default|GetGridSpacing))) 0.0) (LocalVariables|GetStartingLocation)) "0, 0, 0" "1.000000,1.000000,1.000000") "AlwaysSpawn" "MultiplyWithRoot" 0 0)
      (Utilities|Array|Add (Variables|Default|GetGridCells) 0))))