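; BP_Projectile is a tower defence projectile that damages the first BP_Enemy it overlaps and then destroys itself.
; The construction script records its spawn transform as the start location.
; Each tick it compares the distance travelled from that start against MaxDistance and destroys itself once out of range.
; Overlaps with other actor types are ignored, and the graphs contain no movement logic.
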(event Collision|EventActorBeginOverlap
  (params (OtherActor :type Actor%20Object%20Reference))
  (bind _asbp_enemy (Utilities|Casting|CastToBP_Enemy OtherActor))
  (Game|Damage|ApplyDamage _asbp_enemy 2.0 0 0)
  (Actor|DestroyActor))

(event EventTick
  (params (DeltaSeconds :type Float%20%28single-precision%29))
  (if (> (Math|Vector|Distance(Vector) (.location (Transformation|GetActorTransform)) (.location (Variables|Default|GetStartLocation))) (Variables|Default|GetMaxDistance))
    (Actor|DestroyActor)))

(fn ConstructionScript
  (Variables|Default|SetStartLocation (Transformation|GetActorTransform)))