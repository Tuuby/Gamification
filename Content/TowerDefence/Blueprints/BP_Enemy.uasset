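; BP_Enemy is a tower defence enemy that marches along negative X and attacks ally buildings.
; Overlapping a BP_AllyBuilding sets it as target; while one is valid, Tick stops movement and applies damage at the attack-speed rate.
; Incoming damage plays a random 2D sound and reduces health; at zero it notifies BP_GridManager with its energy value and destroys itself.
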(event Custom|AnyDamageChild
  (params (DamagedActor :type Actor%20Object%20Reference) (Damage :type Float%20%28single-precision%29) (DamageType :type Damage%20Type%20Object%20Reference) (InstigatedBy :type Controller%20Object%20Reference) (DamageCauser :type Actor%20Object%20Reference))
  (CallFunction|PlayRandomSound))

(event EventBeginPlay
  (EventDispatchers|BindEventtoOnTakeAnyDamage (delegate Custom|AnyDamageChild)))

(event Collision|EventActorEndOverlap
  (params (OtherActor :type Actor%20Object%20Reference))
  (Utilities|Casting|CastToBP_AllyBuilding OtherActor)
  (Variables|Default|SetTarget 0))

(event EventTick
  (params (DeltaSeconds :type Float%20%28single-precision%29))
  (bind _returnvalue (Transformation|GetActorLocation))
  (Utilities|IsValid (Variables|Default|GetTarget)
    (:Is%20Valid
      (bind _output_get (Variables|Default|SetTimeSinceLastAttack (+ DeltaSeconds (Variables|Default|GetTimeSinceLastAttack))))
      (if (> _output_get (/ 1.0 (Variables|Default|GetAttackSpeed)))
        (Game|Damage|ApplyDamage (Variables|Default|GetTarget) (Variables|Default|GetAttackDamage) 0 0)
        (Variables|Default|SetTimeSinceLastAttack 0.0)))
    (:Is%20Not%20Valid
      (Transformation|SetActorLocation (Math|Vector|MakeVector (- (.x _returnvalue) (* DeltaSeconds (Variables|Default|GetMovementSpeed))) (.y _returnvalue) (.z _returnvalue)) false false))))

(event Collision|EventActorBeginOverlap
  (params (OtherActor :type Actor%20Object%20Reference))
  (bind _asbp_ally_building (Utilities|Casting|CastToBP_AllyBuilding OtherActor))
  (Variables|Default|SetTarget _asbp_ally_building))

(event Game|Damage|EventAnyDamage
  (params (Damage :type Float%20%28single-precision%29) (DamageType :type Damage%20Type%20Object%20Reference) (InstigatedBy :type Controller%20Object%20Reference) (DamageCauser :type Actor%20Object%20Reference))
  (bind _output_get (Variables|Default|SetHealthPoints (- (Variables|Default|GetHealthPoints) Damage)))
  (if (<= _output_get 0.0)
    (bind _returnvalue (Actor|GetActorOfClass "/Game/TowerDefence/Blueprints/BP_GridManager.BP_GridManager_C"))
    (Default|NotifyDeath _returnvalue self (Variables|Default|GetEnergyValue))
    (Actor|DestroyActor)))

(fn ConstructionScript)

(fn PlayRandomSound
  (Audio|PlaySound2D (.OutItem (Utilities|Array|Random (Variables|Default|GetSoundsArray))) 1.0 1.0 0.01 0 0))