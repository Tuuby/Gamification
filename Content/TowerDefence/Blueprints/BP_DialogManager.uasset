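; Dialog manager actor for the tower defence game that shows and removes dialog widgets keyed by a level state ID.
; Separate functions create standard, capture and generic dialog widgets, pass in the state, store the result as ShownDialog and add it to the viewport.
; The capture variant first moves CaptureObject to a transform picked by capture ID from CaptureTransforms.
; RemoveDialogWidget detaches and clears the shown dialog; the event graph is empty.
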(event EventBeginPlay)

(event Collision|EventActorBeginOverlap
  (params (OtherActor :type Actor%20Object%20Reference)))

(event EventTick
  (params (DeltaSeconds :type Float%20%28single-precision%29)))

(fn ConstructionScript)

(fn ShowDialogWidget
  (params (LevelStateID :type Integer))
  (Variables|Default|SetDialogID LevelStateID)
  (bind _returnvalue (UserInterface|CreateWidget "/Game/TowerDefence/UI/Widget_Dialog.Widget_Dialog_C"))
  (Variables|/Game/TowerDefence/UI/Widget_Dialog.Widget_Dialog_C|SetLevelState _returnvalue (Variables|Default|GetDialogID))
  (Variables|Default|SetShownDialog _returnvalue)
  (UserInterface|Viewport|AddtoViewport _returnvalue 2))

(fn ShowCaptureDialogWidget
  (params (LevelStateID :type Integer) (CaptureID :type Integer))
  (Variables|Default|SetDialogID LevelStateID)
  (Transformation|SetActorTransform (Variables|Default|GetCaptureObject) (Utilities|Array|Get(acopy) (Variables|Default|GetCaptureTransforms) CaptureID))
  (bind _returnvalue (UserInterface|CreateWidget "/Game/TowerDefence/UI/Widget_CaptureDialog.Widget_CaptureDialog_C"))
  (Variables|/Game/TowerDefence/UI/Widget_CaptureDialog.Widget_CaptureDialog_C|SetLevelState _returnvalue (Variables|Default|GetDialogID))
  (Variables|Default|SetShownDialog _returnvalue)
  (UserInterface|Viewport|AddtoViewport _returnvalue 2))

(fn RemoveDialogWidget
  (Widget|RemovefromParent (Variables|Default|GetShownDialog))
  (Variables|Default|SetShownDialog 0))

(fn ShowGenericDialogWidget
  (params (LevelStateID :type Integer))
  (bind _returnvalue (UserInterface|CreateWidget "/Game/TowerDefence/UI/Widget_GenericDialog.Widget_GenericDialog_C"))
  (Variables|/Game/TowerDefence/UI/Widget_GenericDialog.Widget_GenericDialog_C|SetLevelState _returnvalue LevelStateID)
  (Variables|Default|SetShownDialog _returnvalue)
  (UserInterface|Viewport|AddtoViewport _returnvalue 2))