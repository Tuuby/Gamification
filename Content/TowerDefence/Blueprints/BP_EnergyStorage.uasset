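; BP_EnergyStorage is a tower defence energy storage building that triggers a kill effect when destroyed.
; On BeginPlay it spawns a BP_EnergyStorageKillArea at an offset from itself and keeps the reference.
; When destroyed, it tells that area to kill enemies and notifies the BP_GridManager that an energy storage was lost.
; It also exposes the world position of its SignalOutput component through GetOutputLocation.
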(event EventBeginPlay
  (bind _returnvalue (Transformation|GetActorTransform))
  (bind _returnvalue_2 (Game|SpawnActorfromClass "/Game/TowerDefence/Blueprints/BP_EnergyStorageKillArea.BP_EnergyStorageKillArea_C" (Math|Transform|MakeTransform (+ (Variables|Default|GetAreaSpawnPoint) (.location _returnvalue)) (.rotation _returnvalue) (.scale _returnvalue)) "Undefined" "MultiplyWithRoot" 0 0))
  (Variables|Default|SetKillArea _returnvalue_2))

(event EventDestroyed
  (Default|KillEnemies (Variables|Default|GetKillArea))
  (bind _returnvalue (Actor|GetActorOfClass "/Game/TowerDefence/Blueprints/BP_GridManager.BP_GridManager_C"))
  (Default|LooseEnergyStorage _returnvalue))

(fn ConstructionScript)

(fn GetOutputLocation
  (return (Transformation|GetWorldLocation (Variables|Default|GetSignalOutput))))