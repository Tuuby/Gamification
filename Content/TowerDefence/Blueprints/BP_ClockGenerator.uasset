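; BP_ClockGenerator is a tower defence actor that acts as a clock source, toggling the boolean signal on its SignalOutput component.
; Tick accumulates delta time and inverts the signal through UpdateSignal once the total exceeds half a period of Frequency.
; TimeSinceLast is never reset in this graph, so after that first threshold the signal flips every tick.
; GetOutputLocation exposes the output component's world location.
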(event EventBeginPlay)

(event Collision|EventActorBeginOverlap
  (params (OtherActor :type Actor%20Object%20Reference)))

(event EventTick
  (params (DeltaSeconds :type Float%20%28single-precision%29))
  (bind _output_get (Variables|Default|SetTimeSinceLast (+ DeltaSeconds (Variables|Default|GetTimeSinceLast))))
  (if (> _output_get (/ 1.0 (* (Variables|Default|GetFrequency) 2.0)))
    (Default|UpdateSignal (Variables|Default|GetSignalOutput) (not (Variables|/Game/TowerDefence/Blueprints/BPC_SignalOutput.BPC_SignalOutput_C|GetSignal (Variables|Default|GetSignalOutput))))))

(fn ConstructionScript)

(fn GetOutputLocation
  (return (Transformation|GetWorldLocation (Variables|Default|GetSignalOutput))))