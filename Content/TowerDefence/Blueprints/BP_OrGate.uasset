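; BP_OrGate is a logic gate in the TowerDefence game that combines two input signals with a boolean OR.
; Each tick, EvaluateSignals reads the Signal values of Input1 and Input2.
; The result is compared with the cached PreviousSignal and passed to the output (spelled "Ouput") through UpdateSignal only when it changes.
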(event EventBeginPlay)

(event Collision|EventActorBeginOverlap
  (params (OtherActor :type Actor%20Object%20Reference)))

(event EventTick
  (params (DeltaSeconds :type Float%20%28single-precision%29))
  (bind _newsignal (CallFunction|EvaluateSignals))
  (if (!= _newsignal (Variables|Default|GetPreviousSignal))
    (Variables|Default|SetPreviousSignal _newsignal)
    (Default|UpdateSignal (Variables|Default|GetOuput) _newsignal)))

(fn ConstructionScript)

(fn EvaluateSignals
  (return (or (Variables|/Game/TowerDefence/Blueprints/BPC_SignalInput.BPC_SignalInput_C|GetSignal (Variables|Default|GetInput1)) (Variables|/Game/TowerDefence/Blueprints/BPC_SignalInput.BPC_SignalInput_C|GetSignal (Variables|Default|GetInput2)))))