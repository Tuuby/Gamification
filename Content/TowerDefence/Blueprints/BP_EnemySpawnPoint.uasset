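; Tower defence spawn point that creates enemies for a row and tracks them in the RowEnemies array.
; SpawnEnemy spawns an enemy at the actor's location regardless of collision, adds it to the array and returns it.
; EnemyDied removes a given enemy from the array, while RemoveSpawn applies fixed damage to every tracked enemy.
; The event graph is unused, so all three functions rely on external callers.
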(event EventBeginPlay)

(event Collision|EventActorBeginOverlap
  (params (OtherActor :type Actor%20Object%20Reference)))

(event EventTick
  (params (DeltaSeconds :type Float%20%28single-precision%29)))

(fn ConstructionScript)

(fn SpawnEnemy
  (bind _returnvalue (Game|SpawnActorfromClass "/Game/TowerDefence/Blueprints/BP_Enemy.BP_Enemy_C" (Math|Transform|MakeTransform (Transformation|GetActorLocation) "0, 0, 0" "1.000000,1.000000,1.000000") "AlwaysSpawn" "MultiplyWithRoot" 0 0))
  (Utilities|Array|Add (Variables|Default|GetRowEnemies) _returnvalue)
  (return _returnvalue))

(fn EnemyDied
  (params (Enemy :type BP%20Enemy%20Object%20Reference))
  (Utilities|Array|RemoveItem (Variables|Default|GetRowEnemies) Enemy))

(fn RemoveSpawn
  (for _array_element (Variables|Default|GetRowEnemies)
    (Game|Damage|ApplyDamage _array_element 1e+02 0 0)))